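; A player-controlled missile launcher rig that fires MissileBP projectiles and returns possession to the Player on right mouse.
; Keyboard axes slide a Sphere reticle relative to the camera, another axis raises or lowers the firing Plane, and Mouse X rotates LookAt.
; Jump launches a missile aimed at the reticle.
; Fire checks GameModeBP's Money, calls MakeBank and launches a faster homing missile, while H calls MakeBank alone.
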(event `InputAction|Jump`
  (params (Key :type "Key Structure"))
  ;[1 1 1] Manual Firing of Missiles
  (:`Pressed`
    (bind _returnvalue (`|SpawnActorFromClass` "/Game/BP/MissileBP.MissileBP_C" (`KismetMathLibrary.MakeTransform` (+ (`self.K2_GetActorLocation`) (0.0 0.0 300.0))) "Undefined" "OverrideRootScale" null null))
    (set `/Game/BP/MissileBP.move_speed` 2000.0 _returnvalue)
    (`self.K2_SetActorRotation` _returnvalue (`KismetMathLibrary.FindLookAtRotation` (`self.K2_GetActorLocation` _returnvalue) (`SceneComponent.K2_GetComponentLocation` (`self.Sphere`))) false)))

(event `InputAxis|Keyboard X`
  (params (AxisValue :type "Float (single-precision)"))
  (bind _returnvalue (`GameplayStatics.GetWorldDeltaSeconds`))
  (bind _camera1 (`self.Camera1`))
  ;[1 1 1] Reticle Movement
  (`SceneComponent.K2_AddLocalOffset` (`self.Sphere`) (* (+ (* (`SceneComponent.GetRightVector` _camera1) (* AxisValue _returnvalue 300.0)) (* (`SceneComponent.GetForwardVector` _camera1) (* (stale `InputAxis|Keyboard Y` AxisValue) _returnvalue 300.0))) (1.0 1.0 0.0)) false false :!label _label))

(event `InputAxis|Keyboard Y`
  (params (AxisValue :type "Float (single-precision)"))
  ;[1 1 1] Reticle Movement
  (goto _label))

(event `InputAxis|Plane Y`
  (params (AxisValue :type "Float (single-precision)"))
  ;[1 1 1] Raise/Lower Firing Plane
  (`SceneComponent.K2_AddLocalOffset` (`self.plane`) (`KismetMathLibrary.MakeVector` 0.0 0.0 (* AxisValue (`GameplayStatics.GetWorldDeltaSeconds`) 600.0)) false false))

(event `self.ReceiveBeginPlay`
  (`self.EnableInput` (`GameplayStatics.GetPlayerController` 0)))

(event `InputAxis|Mouse X`
  (params (AxisValue :type "Float (single-precision)"))
  ;[1 1 1] Camera Control
  (`SceneComponent.K2_AddLocalRotation` (`self.lookAt`) (`KismetMathLibrary.Conv_VectorToRotator` (`KismetMathLibrary.CreateVectorFromYawPitch` AxisValue 0.0 0.5)) false false))

(event `Key|RightMouseButton`
  (params (Key :type "Key Structure"))
  ;[1 1 1] Escape Launcher
  (:`Pressed`
    (`Controller.Possess` (`GameplayStatics.GetPlayerController` 0) (`self. player`))))

(event `InputAction|Fire`
  (params (Key :type "Key Structure"))
  ;[1 1 1] Homing Missiles
  (:`Pressed`
    (bind _asgame_mode_bp (cast `/Game/GameModeBP` (`GameplayStatics.GetGameMode`)))
    (if (>= (`/Game/GameModeBP.money` _asgame_mode_bp) 100)
      (`/Game/GameModeBP.makeBank` _asgame_mode_bp false)
      (bind _returnvalue (`|SpawnActorFromClass` "/Game/BP/MissileBP.MissileBP_C" (`KismetMathLibrary.MakeTransform` (+ (`self.K2_GetActorLocation`) (0.0 0.0 300.0))) "Undefined" "OverrideRootScale" null null))
      (set `/Game/BP/MissileBP.move_speed` 5000.0 _returnvalue)
      (set `/Game/BP/MissileBP.homing` true _returnvalue))))

(event `Key|H`
  (params (Key :type "Key Structure"))
  (:`Pressed`
    (bind _asgame_mode_bp (cast `/Game/GameModeBP` (`GameplayStatics.GetGameMode`)))
    (`/Game/GameModeBP.makeBank` _asgame_mode_bp false)))

(fn `UserConstructionScript`)