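; Spawner actor that builds the voxel battlefield and periodically launches enemy missiles at it.
; BeginPlay lays a sine-wave height grid of VoxelBP, attaches the base to the center voxel, and line-traces down around a ring to attach launchers to the voxels hit.
; Tick runs a frame-count countdown, spawning Enemy-tagged missiles high above random grid points, aimed at other random points and registered in GameModeBP's Missiles array.
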(event `self.ReceiveBeginPlay`
  (bind _launch_spacing (`self.launch_spacing`))
  (for _index (range (* (`self.width`) -1) (+ (`self.width`) 1))
    (for _index_2 (range (* (`self.height`) -1) (+ (`self.height`) 1))
      (bind _loc (`self.GetLocation` _index _index_2))
      (bind _returnvalue (`|SpawnActorFromClass` "/Game/BP/VoxelBP.VoxelBP_C" (`KismetMathLibrary.MakeTransform` _loc) "Undefined" "OverrideRootScale" null null))
      (if (and (== _index 0) (== _index_2 0))
        (bind _returnvalue_2 (`|SpawnActorFromClass` "/Game/BP/BaseBP.BaseBP_C" (`KismetMathLibrary.MakeTransform` (+ _loc (0.0 0.0 140.0))) "Undefined" "OverrideRootScale" _returnvalue null))
        (`self.K2_AttachToActor` _returnvalue_2 _returnvalue "None" "KeepRelative" "KeepRelative" "KeepRelative" true)
        (`PrimitiveComponent.SetConstraintMode` (`/Game/BP/VoxelBP.ground_cube_ground_cube` _returnvalue) "SixDOF"))))
  ;[1 1 1] Launchers
  (for _index_3 (range 1 (+ (`self.num_launchers`) 1))
    (bind _returnvalue_3 (* (/ 360.0 (`KismetMathLibrary.Conv_IntToDouble` (`self.num_launchers`))) (`KismetMathLibrary.Conv_IntToDouble` _index_3)))
    (bind _returnvalue_4 (+ (`self.K2_GetActorLocation`) (`KismetMathLibrary.MakeVector` (* (`KismetMathLibrary.DegSin` _returnvalue_3) _launch_spacing) (* (`KismetMathLibrary.DegCos` _returnvalue_3) _launch_spacing) 100.0)))
    (bind _outhit (`KismetSystemLibrary.LineTraceSingle` :`Start` _returnvalue_4 :`End` (+ _returnvalue_4 (0.0 0.0 -1000.0)) :`TraceChannel` "TraceTypeQuery1" :`DrawTime` 0.0))
    (bind (_bblockinghit _binitialoverlap _time _distance _location _impactpoint _normal _impactnormal _physmat _hitactor) (`GameplayStatics.BreakHitResult` _outhit))
    (bind _returnvalue_5 (`|SpawnActorFromClass` "/Game/BP/LauncherBP.LauncherBP_C" (`KismetMathLibrary.MakeTransform` (+ (`self.K2_GetActorLocation` _hitactor) (0.0 0.0 200.0))) "Undefined" "OverrideRootScale" _hitactor null))
    (`self.K2_AttachToActor` _returnvalue_5 _hitactor "None" "KeepWorld" "KeepWorld" "KeepWorld" true)))

(event `self.ReceiveTick`
  (params (DeltaSeconds :type "Float (single-precision)"))
  ;[1 1 1] Spawns Enemy Missiles
  (bind _result (`/Engine/EditorBlueprintResources/StandardMacros.DecrementFloat` (`self.time_til_missile`))
    (:`  `
      (bind _output_get (set `self.time_til_missile` _result))
      (if (<= _output_get 0.0)
        (set `self.time_til_missile` 200.0)
        (bind (_x _y) (`self.getRandomVoxelTarget`))
        ;;[1 1 1] Point at Random Voxel
        (bind (_x_2 _y_2) (`self.getRandomVoxelTarget`))
        (bind _returnvalue (`KismetMathLibrary.Conv_IntToDouble` _x))
        (bind _returnvalue_2 (`KismetMathLibrary.Conv_IntToDouble` _y))
        (bind _returnvalue_3 (`|SpawnActorFromClass` "/Game/BP/MissileBP.MissileBP_C" (`KismetMathLibrary.MakeTransform` (`KismetMathLibrary.MakeVector` _returnvalue _returnvalue_2 4000.0) (`KismetMathLibrary.FindLookAtRotation` (`KismetMathLibrary.MakeVector` _returnvalue _returnvalue_2 4000.0) (`KismetMathLibrary.MakeVector` (`KismetMathLibrary.Conv_IntToDouble` _x_2) (`KismetMathLibrary.Conv_IntToDouble` _y_2)))) "Undefined" "OverrideRootScale" null null))
        (`KismetArrayLibrary.Array_Add` (`Actor.Tags` _returnvalue_3) "Enemy")
        (bind _asgame_mode_bp (cast `/Game/GameModeBP` (`GameplayStatics.GetGameMode`)))
        (`KismetArrayLibrary.Array_Add` (`/Game/GameModeBP.missiles` _asgame_mode_bp) _returnvalue_3)))))

(fn `GetLocation`
  (params (x :type Integer) (y :type Integer))
  (returns (loc :type "Vector Structure"))
  (return (`KismetMathLibrary.MakeVector` (`KismetMathLibrary.Conv_IntToDouble` (* x 200)) (`KismetMathLibrary.Conv_IntToDouble` (* y 200)) (* (+ (`KismetMathLibrary.Sin` (* x 0.5)) (`KismetMathLibrary.Sin` (* y 0.5))) 50.0))))

(fn `getRandomVoxelTarget`
  (returns (X :type Integer) (Y :type Integer))
  (bind _width (`self.width`))
  (bind _height (`self.height`))
  (return (* (`KismetMathLibrary.RandomIntegerInRange` (* _width -1) _width) 200) (* (`KismetMathLibrary.RandomIntegerInRange` (* _height -1) _height) 200)))

(fn `UserConstructionScript`)