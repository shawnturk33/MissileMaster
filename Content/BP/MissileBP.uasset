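; Missile actor that flies forward, explodes on voxel terrain and intercepts enemy missiles.
; On spawn it claims the nearest missile from GameModeBP's list and, if Homing, turns toward it each tick.
; Voxel contact activates AoE, which damages the base, turns voxels into physics debris, restarts the level on player overlap and fires a radial impulse.
; Hitting an Enemy-tagged missile destroys both and spawns MoneyBP.
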(event `self.ReceiveBeginPlay`
  (`ActorComponent.Deactivate` (`self.AoE`))
  (bind _currmissiletarget1 (`self.findMissileTarget` (`self.K2_GetActorLocation`)))
  (bind _output_get (set `self.target` _currmissiletarget1))
  (`KismetSystemLibrary.PrintString` (`KismetSystemLibrary.GetDisplayName` _output_get)))

(event `self.ReceiveTick`
  (params (DeltaSeconds :type "Float (single-precision)"))
  (bind _target (`self.target`))
  (`self.K2_AddActorLocalOffset` (* (`KismetMathLibrary.Vector_Forward`) (* (`self.move_speed`) (`GameplayStatics.GetWorldDeltaSeconds`))))
  ;[1 1 1] Homing Target
  (if (`self.homing`)
    (if (`KismetSystemLibrary.IsValid` _target)
      (`self.K2_SetActorRotation` (`KismetMathLibrary.FindLookAtRotation` (`self.K2_GetActorLocation`) (`self.K2_GetActorLocation` _target))))))

(event `self.Capsule.OnComponentBeginOverlap`
  (params (OverlappedComponent :type "PrimitiveComponent Object Reference") (OtherActor :type "Actor Object Reference") (OtherComp :type "PrimitiveComponent Object Reference") (OtherBodyIndex :type Integer) (bFromSweep :type Boolean) (SweepResult :type "HitResult Structure (by ref)"))
  (cast `/Game/BP/VoxelBP` OtherActor
    (:`then`
      (`ActorComponent.Activate` (`self.AoE`) false))
    (:`CastFailed`
      (bind _asmissile_bp (cast `/Game/BP/MissileBP` OtherActor))
      (if (`self.ActorHasTag` _asmissile_bp "Enemy")
        (`KismetSystemLibrary.PrintString` "missile collide")
        (`self.K2_DestroyActor` _asmissile_bp)
        (`|SpawnActorFromClass` "/Game/BP/MoneyBP.MoneyBP_C" (`KismetMathLibrary.MakeTransform` (`self.K2_GetActorLocation`)) "AlwaysSpawn" "OverrideRootScale" null null)
        (`self.K2_DestroyActor`)))))

(event `self.AoE.OnComponentActivated`
  (params (Component :type "ActorComponent Object Reference") (bReset :type Boolean))
  (for _array_element (`PrimitiveComponent.GetOverlappingActors` (`self.AoE`) null)
    (if (== (`GameplayStatics.GetObjectClass` _array_element) "/Game/BP/BaseBP.BaseBP_C")
      (bind _asgame_mode_bp (cast `/Game/GameModeBP` (`GameplayStatics.GetGameMode`)))
      (`/Game/GameModeBP.takeDamage` _asgame_mode_bp)
      (elif (== (`GameplayStatics.GetObjectClass` _array_element) "/Game/BP/VoxelBP.VoxelBP_C")
        (bind _asvoxel_bp (cast `/Game/BP/VoxelBP` _array_element))
        (bind _ground_cube_ground_cube (`/Game/BP/VoxelBP.ground_cube_ground_cube` _asvoxel_bp))
        (`SceneComponent.SetWorldScale3D` _ground_cube_ground_cube (0.9 0.9 0.9))
        (`PrimitiveComponent.SetSimulatePhysics` _ground_cube_ground_cube true)
        (`PrimitiveComponent.SetEnableGravity` _ground_cube_ground_cube true)
        (elif (== (`GameplayStatics.GetObjectClass` _array_element) "/Game/BP/PlayerBP.PlayerBP_C")
          (`KismetSystemLibrary.ExecuteConsoleCommand` "RestartLevel" null)))))
  (`RadialForceComponent.FireImpulse` (`self.RadialForce`))
  (`self.K2_DestroyActor`))

(fn `findMissileTarget`
  (params (spawnPos :type "Vector Structure"))
  (returns (currMissileTarget1 :type "/Game/BP/MissileBP Object Reference"))
  (locals (currSmallestDist :type "Float (double-precision)" :default 100000.0) (currMissileTarget :type "/Game/BP/MissileBP Object Reference"))
  (bind _currmissiletarget (`local.currMissileTarget`))
  (bind _asgame_mode_bp (cast `/Game/GameModeBP` (`GameplayStatics.GetGameMode`)))
  (for _array_element (`/Game/GameModeBP.missiles` _asgame_mode_bp)
    (bind _returnvalue (`KismetMathLibrary.Vector_Distance` spawnPos (`SceneComponent.K2_GetComponentLocation` (`Actor.RootComponent` _array_element))))
    (if (<= _returnvalue (`local.currSmallestDist`))
      (set `local.currSmallestDist` _returnvalue)
      (set `local.currMissileTarget` _array_element)))
  (bind _asgame_mode_bp_2 (cast `/Game/GameModeBP` (`GameplayStatics.GetGameMode`)))
  (`KismetArrayLibrary.Array_RemoveItem` (`/Game/GameModeBP.missiles` _asgame_mode_bp_2) _currmissiletarget)
  (return _currmissiletarget))

(fn `UserConstructionScript`)