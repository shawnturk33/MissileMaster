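; Game mode that owns the player's money and HP and manages the HUD, main menu and pause state.
; On BeginPlay it creates the in-game UI, layers the main menu above it, pauses the game and plays the title fade.
; Its functions adjust money and health in fixed steps, writing straight to the HUD text.
; Others toggle launcher tooltips, or switch pause together with the menu buttons and mouse cursor.
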(event `self.ReceiveBeginPlay`
  (bind _main_menu_widget (`self.main_menu_widget`))
  (bind _returnvalue (`|CreateWidget` "/Game/Meshes/menu/in_game_ui.in_game_ui_C"))
  (bind _output_get (set `self.ui_widget` _returnvalue))
  (`UserWidget.AddToViewport` _output_get 0)
  (bind _returnvalue_2 (`|CreateWidget` "/Game/Meshes/menu/main_menu_ui.main_menu_ui_C"))
  (bind _output_get_2 (set `self.main_menu_widget` _returnvalue_2))
  (`UserWidget.AddToViewport` _output_get_2 1)
  (set `PlayerController.bShowMouseCursor` true (`GameplayStatics.GetPlayerController` 0))
  (`self.pauseGame` true)
  (`UserWidget.PlayAnimation` _main_menu_widget (`/Game/Meshes/menu/main_menu_ui.TitleFadeAnimation` _main_menu_widget) 0.0 1 "Forward" 1.0))

(fn `dontShowLauncherTooltips`
  (`Widget.SetVisibility` (`/Game/Meshes/menu/in_game_ui.HealText` (`self.ui_widget`)) "Collapsed")
  (`Widget.SetVisibility` (`/Game/Meshes/menu/in_game_ui.AutoFireText` (`self.ui_widget`)) "Collapsed"))

(fn `makeBank`
  (params (`deposit?` :type Boolean))
  (locals (NewLocalVar_0 :type Integer :default 0))
  (if `deposit?`
    (bind _output_get (set `self.money` (+ (`self.money`) 100)))
    (`TextBlock.SetText` (`/Game/Meshes/menu/in_game_ui.money` (`self.ui_widget`)) (`KismetTextLibrary.Conv_IntToText` _output_get))
    (else
      (bind _output_get_2 (set `self.money` (- (`self.money`) 100)))
      (`TextBlock.SetText` (`/Game/Meshes/menu/in_game_ui.money` (`self.ui_widget`)) (`KismetTextLibrary.Conv_IntToText` _output_get_2)))))

(fn `pauseGame`
  (params (pauseBool :type Boolean))
  (bind _returnvalue (`GameplayStatics.GetPlayerController` 0))
  (if pauseBool
    (`Widget.SetVisibility` (`/Game/Meshes/menu/in_game_ui.ResumeButton` (`self.ui_widget`)) "Visible")
    (`Widget.SetVisibility` (`/Game/Meshes/menu/in_game_ui.QuitButton` (`self.ui_widget`)) "Visible")
    (`Widget.SetVisibility` (`/Game/Meshes/menu/in_game_ui.NewGameButton` (`self.ui_widget`)) "Visible")
    (set `PlayerController.bShowMouseCursor` true _returnvalue)
    (`GameplayStatics.SetGamePaused` true)
    (else
      (`Widget.SetVisibility` (`/Game/Meshes/menu/in_game_ui.ResumeButton` (`self.ui_widget`)) "Collapsed")
      (`Widget.SetVisibility` (`/Game/Meshes/menu/in_game_ui.QuitButton` (`self.ui_widget`)) "Collapsed")
      (`Widget.SetVisibility` (`/Game/Meshes/menu/in_game_ui.NewGameButton` (`self.ui_widget`)) "Collapsed")
      (set `PlayerController.bShowMouseCursor` false _returnvalue)
      (`GameplayStatics.SetGamePaused` false))))

(fn `showLauncherTooltips`
  (`Widget.SetVisibility` (`/Game/Meshes/menu/in_game_ui.HealText` (`self.ui_widget`)) "Visible")
  (`Widget.SetVisibility` (`/Game/Meshes/menu/in_game_ui.AutoFireText` (`self.ui_widget`)) "Visible"))

(fn `takeDamage`
  (bind _output_get (set `self.hp` (- (`self.hp`) 10.0)))
  (`TextBlock.SetText` (`/Game/Meshes/menu/in_game_ui.HP` (`self.ui_widget`)) (`KismetTextLibrary.Conv_DoubleToText` _output_get "HalfToEven")))

(fn `UserConstructionScript`)